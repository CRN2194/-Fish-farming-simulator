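; Drivable boat pawn with a zoomable follow camera, an enter capsule for taking control and a box that teleports interacting actors to an arrow.
; Server events store axis inputs and fire uncontrolled cannons; Tick turns inputs into mass-scaled physics forces, with steering applied at an offset point.
; Tick also spawns wakes by distance travelled near BP_Ocean height.
; Construction script configures mesh, optional separate pawn collision, center of mass and capsule.
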(event OnComponentEndOverlap(EnterCapsule)
  (params (OverlappedComponent :type Primitive%20Component%20Object%20Reference) (OtherActor :type Actor%20Object%20Reference) (OtherComp :type Primitive%20Component%20Object%20Reference) (OtherBodyIndex :type Integer))
  ;[1 1 1] EnterCapsule
  (Utilities|SetInterractionVolume OtherActor (Variables|Default|GetEnterCapsule) false))

(event OnComponentBeginOverlap(Box)
  (params (OverlappedComponent :type Primitive%20Component%20Object%20Reference) (OtherActor :type Actor%20Object%20Reference) (OtherComp :type Primitive%20Component%20Object%20Reference) (OtherBodyIndex :type Integer) (bFromSweep :type Boolean) (SweepResult :type Hit%20Result%20Structure%20%28by%20ref%29))
  (Utilities|SetInterractionVolume OtherActor (Variables|Default|GetBox) true))

(event OnComponentEndOverlap(Box)
  (params (OverlappedComponent :type Primitive%20Component%20Object%20Reference) (OtherActor :type Actor%20Object%20Reference) (OtherComp :type Primitive%20Component%20Object%20Reference) (OtherBodyIndex :type Integer))
  (Utilities|SetInterractionVolume OtherActor (Variables|Default|GetBox) false))

(event OnComponentBeginOverlap(EnterCapsule)
  (params (OverlappedComponent :type Primitive%20Component%20Object%20Reference) (OtherActor :type Actor%20Object%20Reference) (OtherComp :type Primitive%20Component%20Object%20Reference) (OtherBodyIndex :type Integer) (bFromSweep :type Boolean) (SweepResult :type Hit%20Result%20Structure%20%28by%20ref%29))
  ;[1 1 1] EnterCapsule
  (Utilities|SetInterractionVolume OtherActor (Variables|Default|GetEnterCapsule) true))

(event Custom|ServerCannonFire
  ;[0.15 0.05 0.05 0.5] Server: fire cannons
  (for _array_element (Variables|Default|GetCannonsArray)
    (Utilities|IsValid _array_element
      (:Is%20Valid
        (if (not (Class|Pawn|IsControlled _array_element))
          (Default|Fire! _array_element))))))

(event Custom|ServerMoveRight
  (params (Value :type Float%20%28single-precision%29))
  ;[0.15 0.05 0.05 0.5] Server: set axis values and replicate
  (Variables|Default|SetRightAxisValue Value))

(event Custom|ServerMoveForward
  (params (Value :type Float%20%28single-precision%29))
  ;[0.15 0.05 0.05 0.5] Server: set axis values and replicate
  (Variables|Default|SetForwardAxisValue Value))

(event EventPossessed
  (params (NewController :type Controller%20Object%20Reference))
  (bind _cameraspringarm (Variables|Default|GetCameraSpringArm))
  (bind _returnvalue (Transformation|GetWorldRotation _cameraspringarm))
  (Utilities|FlowControl|Delay 0.05)
  (Pawn|SetControlRotation NewController (Math|Rotator|MakeRotator 0.0 (.pitch _returnvalue) (.yaw _returnvalue)))
  (Variables|/Script/Engine.SpringArmComponent|SetTargetArmLength (Variables|Default|GetCameraSpringArm) 5e+02))

(event EventTick
  (params (DeltaSeconds :type Float%20%28single-precision%29))
  (bind _staticmesh (Variables|Default|GetStaticMesh))
  (bind _wakeemitter (Variables|Default|GetWakeEmitter))
  (bind _staticmesh_2 (Variables|Default|GetStaticMesh))
  (bind _staticmesh_3 (Variables|Default|GetStaticMesh))
  (bind _steerforcelocation (Variables|Default|GetSteerForceLocation))
  (bind _returnvalue (Transformation|GetWorldRotation _staticmesh_3))
  (bind _returnvalue_2 (Physics|GetMass _staticmesh_2))
  (bind _returnvalue_3 (Transformation|GetWorldLocation _wakeemitter))
  (bind _returnvalue_4 (Math|Vector2D|MakeVector2D (.x _returnvalue_3) (.y _returnvalue_3)))
  ;[0.9619 1 0.4097 0.743] Tick
  (Utilities|FlowControl|Sequence
    (:then_0
      ;[1 1 1] Camera Zoom in/out
      (Utilities|CameraZoom (Variables|Default|GetCameraSpringArm) 1e+03 2.4e+04 1e+02 5.0 0.0
        (:Exit
          ;[1 1 1] Camera rotation
          (Pawn|Input|AddControllerYawInput (* (- (.yaw _returnvalue) (Variables|Default|GetPrevYaw)) 0.4))
          (Variables|Default|SetPrevYaw (.yaw _returnvalue)))))
    (:then_1
      ;[0.4508 1 0.4793 0.646] Apply movement forward/right forces
      (Class|PrimitiveComponent|AddForceatLocation _staticmesh (* (Math|Vector|GetRightVector (Transformation|GetWorldRotation _steerforcelocation)) (* _returnvalue_2 (Variables|Default|GetSteeringSpeed) (Variables|Default|GetRightAxisValue))) (Transformation|GetWorldLocation _steerforcelocation) "None")
      (Physics|AddForce _staticmesh (* (Math|Vector|GetForwardVector _staticmesh_2) (* _returnvalue_2 (Variables|Default|GetForwardSpeed) (Variables|Default|GetForwardAxisValue))) "None" false))
    (:then_2
      ;[1 1 1] Wakes Test
      (if (Variables|Default|GetSpawnWake)
        (if (> (Math|Vector|VectorLength (Transformation|GetVelocity)) 3e+02)
          (if (>= (Math|Vector2D|Vector2DLength (- _returnvalue_4 (Variables|Default|GetLastPos))) 7e+02)
            (bind _output_get (Variables|Default|SetLastPos _returnvalue_4))
            (bind _outactors (Actor|GetAllActorsOfClass "/Game/Ocean/BP_Ocean.BP_Ocean_C"))
            (Utilities|IsValid (Utilities|Array|Get(acopy) _outactors)
              (:Is%20Valid
                (if (Math|Float|InRange(Float) (.z _returnvalue_3) (- (.z (Transformation|GetActorLocation (Utilities|Array|Get(acopy) _outactors))) 3.5e+02) (+ (.z (Transformation|GetActorLocation (Utilities|Array|Get(acopy) _outactors))) 1e+02))
                  (Game|SpawnActorfromClass "/Game/Ocean/FoamWakes/BP_Wake.BP_Wake_C" (Math|Transform|MakeTransform (Math|Vector|MakeVector (.x _output_get) (.y _output_get) (.z (Transformation|GetActorLocation (Utilities|Array|Get(acopy) _outactors)))) (Math|Rotator|MakeRotator 0.0 0.0 (.yaw (Transformation|GetWorldRotation (Variables|Default|GetWakeEmitter)))) "1,1,1") "AlwaysSpawn" 0 0))))))))))

(event EventTryInteract
  (params (Actor :type Pawn%20Object%20Reference))
  ;[1 1 1] Send controller request to drive
  (if (Collision|IsOverlappingActor (Variables|Default|GetEnterCapsule) Actor :!class /Script/Engine.PrimitiveComponent)
    (Class|InteractInterface|TryEnterVehicle(Message) (Pawn|GetController Actor) self)
    (else
      ;[1 1 1] Teleport box
      (if (Collision|IsOverlappingActor (Variables|Default|GetBox) Actor :!class /Script/Engine.PrimitiveComponent)
        (Transformation|SetActorLocation Actor (Transformation|GetWorldLocation (Variables|Default|GetArrow)) false true)))))

(event Input|MouseEvents|MouseWheelDown
  (params (Key :type Key%20Structure))
  (bind _staticmesh (Variables|Default|GetStaticMesh))
  (bind _returnvalue (Transformation|GetWorldRotation _staticmesh))
  ;[1 1 1] Camera Zoom in/out
  (:Released
    (Utilities|CameraZoom (Variables|Default|GetCameraSpringArm) 1e+03 2.4e+04 1e+02 5.0 0.0) ; enters at ZoomOut
  ))

(event Input|MouseEvents|MouseWheelUp
  (params (Key :type Key%20Structure))
  (bind _staticmesh (Variables|Default|GetStaticMesh))
  (bind _returnvalue (Transformation|GetWorldRotation _staticmesh))
  ;[1 1 1] Camera Zoom in/out
  (:Released
    (Utilities|CameraZoom (Variables|Default|GetCameraSpringArm) 1e+03 2.4e+04 1e+02 5.0 0.0) ; enters at ZoomIn
  ))

(fn ConstructionScript
  (bind _staticmesh (Variables|Default|GetStaticMesh))
  (bind _pawncollisionmesh (Variables|Default|GetPawnCollisionMesh))
  (bind _smesh (Variables|Default|GetSMesh))
  (bind _entercapsule (Variables|Default|GetEnterCapsule))
  (Utilities|FlowControl|Sequence
    (:then_0
      (if (and (Variables|Default|GetUseSeperatePawnCollision) (Utilities|IsValid _smesh))
        (Components|StaticMesh|SetStaticMesh _pawncollisionmesh _smesh)
        (else
          (Components|DestroyComponent _pawncollisionmesh)
          (Collision|SetCollisionResponsetoChannel _staticmesh "ECC_Pawn" "ECR_Block")
          (Utilities|IsValid (Variables|Default|GetSMesh)
            (:Is%20Valid
              _))))
      (Components|StaticMesh|SetStaticMesh _staticmesh _smesh))
    (:then_1
      (Class|PrimitiveComponent|SetCenterOfMass (Variables|Default|GetStaticMesh) (Variables|Default|GetCenterOfMassOffset) "None")
      (Transformation|SetRelativeLocationAndRotation _entercapsule (Variables|Default|GetEnterCapsuleLocation) (Variables|Default|GetEnterCapsuleRotation) false false)
      (Components|Capsule|SetCapsuleSize _entercapsule (Variables|Default|GetEnterCapsuleRadius) (Variables|Default|GetEnterCapsuleHeight) false))))