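; BP_Button is an interactable button that registers itself with RobotCharacter_BP while that character is inside its sphere trigger.
; The construction script applies configurable mesh, transform, trigger radius and location, and UI location to its components.
; ToggleUI shows or hides the interaction prompt component.
; Interact stores the interacting character and only prints a Spanish debug message saying E was pressed, with no other button effect.
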(event OnComponentBeginOverlap(InteractTigger)
  (params (OverlappedComponent :type Primitive%20Component%20Object%20Reference) (OtherActor :type Actor%20Object%20Reference) (OtherComp :type Primitive%20Component%20Object%20Reference) (OtherBodyIndex :type Integer) (bFromSweep :type Boolean) (SweepResult :type Hit%20Result%20Structure%20%28by%20ref%29))
  (bind _asrobot_character_bp (Utilities|Casting|CastToRobotCharacter_BP OtherActor))
  (Default|AddInteraction _asrobot_character_bp self))

(event OnComponentEndOverlap(InteractTigger)
  (params (OverlappedComponent :type Primitive%20Component%20Object%20Reference) (OtherActor :type Actor%20Object%20Reference) (OtherComp :type Primitive%20Component%20Object%20Reference) (OtherBodyIndex :type Integer))
  (bind _asrobot_character_bp (Utilities|Casting|CastToRobotCharacter_BP OtherActor))
  (Default|RemoveInteraction _asrobot_character_bp self))

(fn ConstructionScript
  (Setup|SetupMesh)
  (Setup|SetupTrigger)
  (Setup|SetupUI))

(fn SetupMesh
  (bind _interactionmesh (Variables|Default|GetInteractionMesh))
  (Components|StaticMesh|SetStaticMesh _interactionmesh (Variables|Setup|GetInteractMesh))
  (Transformation|SetRelativeTransform _interactionmesh (Variables|Setup|GetMeshTransform) false false))

(fn SetupTrigger
  (bind _interacttigger (Variables|Default|GetInteractTigger))
  (Components|Sphere|SetSphereRadius _interacttigger (Variables|Setup|GetTriggerRadius) true)
  (Transformation|SetRelativeLocation _interacttigger (Variables|Setup|GetTriggerLocation) false false))

(fn SetupUI
  (Transformation|SetRelativeLocation (Variables|Default|GetInteractUI) (Variables|Setup|GetUILocation) false false))

(fn ToggleUI
  (params (visible :type Boolean))
  (Rendering|SetVisibility (Variables|Default|GetInteractUI) visible false))

(fn Interact
  (params (Interact :type Robot%20Character%20BP%20Object%20Reference))
  (Variables|Interact|SetInteractorCharacter Interact)
  (Development|PrintString "Letra E presionada"))