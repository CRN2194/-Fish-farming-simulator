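; Player-controlled robot character that moves, swims on overlapping BP_Ocean, toggles lights and switches between first- and third-person cameras.
; Tick enables buoyancy only while stationary and feeds turn flags to the AnimBP.
; Grab line-traces from the camera and attaches physics objects to the "fish" socket, while M sets a RosPublisher flag.
; A looping timer selects the interactable best aligned with the robot's forward vector by dot product for InCages to trigger.
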(event OnComponentBeginOverlap(SphereCollisionWater)
  (params (OverlappedComponent :type Primitive%20Component%20Object%20Reference) (OtherActor :type Actor%20Object%20Reference) (OtherComp :type Primitive%20Component%20Object%20Reference) (OtherBodyIndex :type Integer) (bFromSweep :type Boolean) (SweepResult :type Hit%20Result%20Structure%20%28by%20ref%29))
  (bind _charactermovement (Variables|Character|GetCharacterMovement))
  (bind _returnvalue (Class|MovementComponent|GetPhysicsVolume _charactermovement))
  ;[1 1 1] UnderWater
  (Utilities|Casting|CastToBP_Ocean OtherActor)
  (Variables|Default|SetSumerged? true)
  (Variables|/Script/Engine.PhysicsVolume|SetbWaterVolume _returnvalue true)
  (Variables|/Script/Engine.PhysicsVolume|SetFluidFriction _returnvalue 5.0)
  (Pawn|Components|CharacterMovement|SetMovementMode _charactermovement "MOVE_Swimming" 0))

(event OnComponentEndOverlap(SphereCollisionWater)
  (params (OverlappedComponent :type Primitive%20Component%20Object%20Reference) (OtherActor :type Actor%20Object%20Reference) (OtherComp :type Primitive%20Component%20Object%20Reference) (OtherBodyIndex :type Integer))
  (bind _charactermovement (Variables|Character|GetCharacterMovement))
  ;[1 1 1] UnderWater
  (Utilities|Casting|CastToBP_Ocean OtherActor)
  (Variables|Default|SetSumerged? false)
  (Variables|/Script/Engine.PhysicsVolume|SetbWaterVolume (Class|MovementComponent|GetPhysicsVolume _charactermovement) false)
  (Pawn|Components|CharacterMovement|SetMovementMode _charactermovement "MOVE_None" 0))

(event Custom|GrabObject
  (bind _returnvalue (Game|GetPlayerCameraManager 0))
  (bind _returnvalue_2 (Transformation|GetActorLocation _returnvalue))
  ;[1 1 1] Grab
  (bind (_outhit _returnvalue_3) (Collision|LineTraceByChannel _returnvalue_2 (+ (* (Transformation|GetActorForwardVector _returnvalue) 300) _returnvalue_2) "TraceTypeQuery1" false 0 "None"))
  (if _returnvalue_3
    (if (Physics|IsSimulatingPhysics (.HitComponent (Collision|BreakHitResult _outhit)) "None")
      (Transformation|AttachComponentToComponent (.HitComponent (Collision|BreakHitResult _outhit)) (Variables|/Script/Engine.Character|GetMesh (Game|GetPlayerCharacter 0)) "fish" "SnapToTarget" "KeepRelative" "KeepRelative" true)
      (Variables|Default|SetGrab? true)
      (Collision|SetCollisionResponsetoChannel (.HitComponent (Collision|BreakHitResult _outhit)) "ECC_Pawn" "ECR_Overlap")
      (Class|PrimitiveComponent|SetAngularDamping (.HitComponent (Collision|BreakHitResult _outhit)) 1e+01))))

(event Custom|ReleaseObject
  ;[1 1 1] Grab
  (Physics|SetSimulatePhysics (.HitComponent (Collision|BreakHitResult (stale Custom|GrabObject _outhit))) true)
  (Variables|Default|SetGrab? false)
  (Transformation|DetachFromActor "KeepWorld" "KeepWorld" "KeepWorld")
  (Collision|SetCollisionResponsetoChannel (.HitComponent (Collision|BreakHitResult (stale Custom|GrabObject _outhit))) "ECC_Pawn" "ECR_Block")
  (Class|PrimitiveComponent|SetAllPhysicsLinearVelocity (.HitComponent (Collision|BreakHitResult (stale Custom|GrabObject _outhit))) "0, 0, 0" false)
  (Utilities|FlowControl|Delay 0.2)
  (Class|PrimitiveComponent|SetAngularDamping (.HitComponent (Collision|BreakHitResult (stale Custom|GrabObject _outhit))) 0.0))

(event EventBeginPlay
  (Utilities|FlowControl|Sequence
    (:then_0
      ;[1 1 1] Time Interect
      (bind _returnvalue (UserInterface|CreateWidget "/Game/Models/Robot/BP_Robot/PrincipalMenu.PrincipalMenu_C" (Game|GetPlayerController 0)))
      (UserInterface|Viewport|AddtoViewport _returnvalue 0)
      (bind _returnvalue_2 (Utilities|Time|SetTimerbyFunctionName 0 "UpdateInteraction" (Variables|Default|GetTime) true))
      (bind _output_get (Variables|Default|SetInteraction _returnvalue_2))
      (Utilities|Time|UnpauseTimerbyHandle _output_get))
    (:then_1
      ;[1 1 1] light
      (if (Variables|Default|GetSwitchLed)
        (Rendering|ToggleVisibility (Variables|Default|GetPointLight) false)
        (Rendering|ToggleVisibility (Variables|Default|GetMiddle) false)
        (Rendering|ToggleVisibility (Variables|Default|GetPointLightRigth) false)
        (Rendering|ToggleVisibility (Variables|Default|GetPointLightLeft) false)))))

(event EventTick
  (params (DeltaSeconds :type Float%20%28single-precision%29))
  (bind _charactermovement (Variables|Character|GetCharacterMovement))
  (bind _mesh (Variables|Character|GetMesh))
  (bind _buoyancy (Variables|Default|GetBuoyancy))
  (bind _mesh_2 (Variables|Character|GetMesh))
  (bind _returnvalue (Class|PawnMovementComponent|GetPawnOwner _charactermovement))
  (bind _returnvalue_2 (Components|SkeletalMesh|GetAnimInstance _mesh))
  (bind _returnvalue_3 (Components|SkeletalMesh|GetAnimInstance _mesh_2))
  (Utilities|FlowControl|Sequence
    (:then_0
      ;[1 1 1] BuoyancyRbt
      (Utilities|IsValid _returnvalue
        (:Is%20Valid
          (bind _output_get (Variables|Default|SetSpeedUnderWater (Math|Vector|VectorLength (Transformation|GetVelocity _returnvalue))))
          (if (> _output_get 0.0)
            (Components|Activation|Deactivate _buoyancy)
            (else
              (Components|Activation|Activate _buoyancy (Variables|Default|GetActivationBuoyancy)))))))
    (:then_1
      ;[1 1 1] Grab
      (Physics|Components|PhysicsHandle|SetTargetLocation (Variables|Default|GetPhysicsHandle) (Transformation|GetWorldLocation (Variables|Default|GetLocation))))
    (:then_2
      ;[1 1 1] Animation TurnRigth
      (if (and (!= (Input|AxisValues|Getturn) 0.0) (!= (Input|AxisValues|Getturn) -1.0))
        (bind _asanim_robot_bp (Utilities|Casting|CastToAnimRobot_BP _returnvalue_3))
        (Variables|/Game/Models/Robot/BP_Robot/AnimRobot_BP.AnimRobot_BP_C|SetTurnRigth _asanim_robot_bp true)
        (else
          (bind _asanim_robot_bp_2 (Utilities|Casting|CastToAnimRobot_BP _returnvalue_3))
          (Variables|/Game/Models/Robot/BP_Robot/AnimRobot_BP.AnimRobot_BP_C|SetTurnRigth _asanim_robot_bp_2 false))))
    (:then_3
      ;[1 1 1] Animation TurnLeft
      (if (and (!= (Input|AxisValues|Getturn) 0.0) (!= (Input|AxisValues|Getturn) 1.0))
        (bind _asanim_robot_bp_3 (Utilities|Casting|CastToAnimRobot_BP _returnvalue_2))
        (Variables|/Game/Models/Robot/BP_Robot/AnimRobot_BP.AnimRobot_BP_C|SetTurnLeft _asanim_robot_bp_3 true)
        (else
          (bind _asanim_robot_bp_4 (Utilities|Casting|CastToAnimRobot_BP _returnvalue_2))
          (Variables|/Game/Models/Robot/BP_Robot/AnimRobot_BP.AnimRobot_BP_C|SetTurnLeft _asanim_robot_bp_4 false))))))

(event Input|ActionEvents|InputActionligth
  (params (Key :type Key%20Structure))
  ;[1 1 1] light
  (:Pressed
    (Variables|Default|SetSwitchLed true)
    (Rendering|ToggleVisibility (Variables|Default|GetPointLight) false)
    (Rendering|ToggleVisibility (Variables|Default|GetMiddle) false)
    (Rendering|ToggleVisibility (Variables|Default|GetPointLightRigth) false)
    (Rendering|ToggleVisibility (Variables|Default|GetPointLightLeft) false)))

(event Input|ActionEvents|InputActionInCages
  (params (Key :type Key%20Structure))
  ;[1 1 1] Active Button Interaction
  (:Pressed
    (bind _selectedinteraction (Variables|Default|GetSelectedInteraction)
      (:then
        (Default|Interact _selectedinteraction self))
      (:else))))

(event Input|ActionEvents|InputActionGrab
  (params (Key :type Key%20Structure))
  ;[1 1 1] Activate Grab
  (:Pressed
    (if (Variables|Default|GetGrab?)
      (CallFunction|ReleaseObject)
      (else
        (CallFunction|GrabObject)))))

(event Input|AxisEvents|InputAxisfordward
  (params (AxisValue :type Float%20%28single-precision%29))
  ;[1 1 1] Move
  (Pawn|Input|AddMovementInput (Math|Vector|GetForwardVector (Pawn|GetControlRotation :!class /Script/Engine.Pawn)) AxisValue false))

(event Input|AxisEvents|InputAxisup-down
  (params (AxisValue :type Float%20%28single-precision%29))
  ;[1 1 1] Direction
  (Pawn|Input|AddMovementInput (Math|Vector|GetForwardVector (Pawn|GetControlRotation :!class /Script/Engine.Pawn)) 0.001 false)
  (Pawn|Input|AddControllerPitchInput (* AxisValue (Variables|Default|Getup_down) (Utilities|Time|GetWorldDeltaSeconds))))

(event Input|AxisEvents|InputAxisside
  (params (AxisValue :type Float%20%28single-precision%29))
  ;[1 1 1] Move
  (Pawn|Input|AddMovementInput (Math|Vector|GetRightVector (Math|Rotator|MakeRotator 0.0 0.0 (.Yaw (Math|Rotator|BreakRotator (Pawn|GetControlRotation :!class /Script/Engine.Pawn))))) AxisValue false))

(event Input|AxisEvents|InputAxisturn
  (params (AxisValue :type Float%20%28single-precision%29))
  ;[1 1 1] Direction
  (Pawn|Input|AddControllerYawInput (* AxisValue (Variables|Default|GetTurn) (Utilities|Time|GetWorldDeltaSeconds))))

(event Input|GamepadEvents|GamepadLeftShoulder
  (params (Key :type Key%20Structure))
  ;[1 1 1] Change camera
  (:Pressed
    (CallFunction|FirstPerson)))

(event Input|GamepadEvents|GamepadLeftStickUp
  (params (Key :type Key%20Structure))
  ;[1 1 1] Change camera
  (:Pressed
    (CallFunction|ThirdPerson)))

(event Input|KeyboardEvents|M
  (params (Key :type Key%20Structure))
  (bind _rospublisher (Variables|Default|GetRosPublisher))
  (:Pressed
    (Variables|/Script/ROSIntegration.RosPublisher|SetestaPresionadoelboton _rospublisher true))
  (:Released
    (Variables|/Script/ROSIntegration.RosPublisher|SetestaPresionadoelboton _rospublisher false)))

(event Input|KeyboardEvents|1
  (params (Key :type Key%20Structure))
  ;[1 1 1] Change camera
  (:Pressed
    (CallFunction|FirstPerson)))

(event Input|KeyboardEvents|2
  (params (Key :type Key%20Structure))
  ;[1 1 1] Change camera
  (:Pressed
    (CallFunction|ThirdPerson)))

(fn ConstructionScript)

(fn FirstPerson
  (Components|Activation|SetActive (Variables|Character|GetFirstPersonC) true false)
  (Components|Activation|SetActive (Variables|Character|GetThirdPersonC) false false)
  (Variables|Default|SetbUseControllerRotationYaw true))

(fn ThirdPerson
  (Components|Activation|SetActive (Variables|Character|GetFirstPersonC) false false)
  (Components|Activation|SetActive (Variables|Character|GetThirdPersonC) true false)
  (Variables|Default|SetbUseControllerRotationYaw true))

(fn AddInteraction
  (params (Interaction :type BP%20Button%20Object%20Reference))
  (bind _interactionlist (Variables|Default|GetInteractionList))
  (Utilities|Array|AddUnique _interactionlist Interaction)
  (if (> (Utilities|Array|Length _interactionlist) 0)
    (Utilities|Time|UnpauseTimerbyHandle (Variables|Default|GetInteraction))
    (else
      (Utilities|Time|PauseTimerbyHandle (Variables|Default|GetInteraction))
      (CallFunction|SetBestInteraction))))

(fn RemoveInteraction
  (params (Interaction :type BP%20Button%20Object%20Reference))
  (bind _interactionlist (Variables|Default|GetInteractionList))
  (Utilities|Array|RemoveItem _interactionlist Interaction)
  (if (> (Utilities|Array|Length _interactionlist) 0)
    (Utilities|Time|UnpauseTimerbyHandle (Variables|Default|GetInteraction))
    (else
      (Utilities|Time|PauseTimerbyHandle (Variables|Default|GetInteraction))
      (CallFunction|SetBestInteraction))))

(fn UpdateInteraction
  (bind _shouldupdate (CallFunction|ShouldUpdateInteraction))
  (if _shouldupdate
    (CallFunction|GetBestInteraction)
    (else
      (CallFunction|SetBestInteraction))))

(fn ShouldUpdateInteraction
  (return (> (Utilities|Array|Length (Variables|Default|GetInteractionList)) 0)))

(fn GetBestInteraction
  (bind _dots (LocalVariables|GetDots))
  (bind (_indexofmaxvalue _maxvalue) (Math|Float|MaxOfFloatArray _dots))
  (for _array_element (Variables|Default|GetInteractionList)
    (Utilities|Array|Add (LocalVariables|GetDots) (Math|Vector|DotProduct (Math|Vector|Normalize (- (Transformation|GetWorldLocation (Variables|/Game/Button/BP_Button.BP_Button_C|GetInteractUI _array_element)) (Transformation|GetActorLocation self))) (Transformation|GetActorForwardVector self))))
  (if (>= _maxvalue (Variables|Default|GetInteractThreshold))
    (CallFunction|SetBestInteraction (Utilities|Array|Get(acopy) (Variables|Default|GetInteractionList) _indexofmaxvalue))
    (else
      (CallFunction|SetBestInteraction))))

(fn SetBestInteraction
  (params (Interaction :type BP%20Button%20Object%20Reference))
  (bind _output_get (LocalVariables|SetNewInteraction Interaction))
  (Utilities|IsValid _output_get
    (:Is%20Valid
      (if (!= (LocalVariables|GetNewInteraction) (Variables|Default|GetSelectedInteraction))
        (bind _selectedinteraction (Variables|Default|GetSelectedInteraction)
          (:then
            (Default|ToggleUI _selectedinteraction false))
          (:else
            _))
        (bind _output_get_2 (Variables|Default|SetSelectedInteraction (LocalVariables|GetNewInteraction)))
        (Default|ToggleUI _output_get_2 true)
        (else
          (bind _selectedinteraction_2 (Variables|Default|GetSelectedInteraction)
            (:then
              (Default|ToggleUI _selectedinteraction_2 false)
              (Variables|Default|SetSelectedInteraction 0))
            (:else)))))))